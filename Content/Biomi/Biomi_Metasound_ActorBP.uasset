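; An actor Blueprint that plays a MetaSound and toggles one of its float parameters from the keyboard.
; On BeginPlay it enables input from the first player controller and starts its Audio component.
; The Enter key drives a FlipFlop and prints the selected value, while Tick pushes one of two fixed values to the "AdditionalOperands 2" parameter every frame based on that state.
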(event `self.ReceiveBeginPlay`
  (`self.EnableInput` (`GameplayStatics.GetPlayerController` 0))
  (`AudioComponent.Play` (`self.Audio`) 0.0))

(event `self.ReceiveTick`
  (params (DeltaSeconds :type "Float (single-precision)"))
  (`AudioParameterControllerInterface.SetFloatParameter` (`self.Audio`) "AdditionalOperands 2" (`KismetMathLibrary.SelectFloat` 440.0 100.0 (stale `Key|Enter` _isa))))

(event `Key|Enter`
  (params (Key :type "Key Structure"))
  (:`Pressed`
    (bind _isa (`/Engine/EditorBlueprintResources/StandardMacros.FlipFlop`)
      (:`A`
        _)
      (:`B`
        _))
    (`KismetSystemLibrary.PrintString` (select `bool` _isa :`false` "100" :`true` "440"))))

(fn `UserConstructionScript`)